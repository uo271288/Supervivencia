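; BP_Weapon is a weapon actor that fires a laser-style projectile when its Shoot event is called.
; Shoot spawns BP_Projectile at the Arrow component's transform, with a short-lived spark emitter at the muzzle and a laser sound at the actor's location.
; A DoOnce reset after a half-second delay limits the fire rate.
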(event Custom|Shoot
  (bind _arrow (Variables|Default|GetArrow))
  (bind _returnvalue (Transformation|GetWorldTransform _arrow))
  (Utilities|FlowControl|DoOnce false :!label _label
    (:Completed
      (Utilities|FlowControl|Sequence
        (:then_0
          (Game|SpawnActorfromClass "/Game/BP_Projectile.BP_Projectile_C" _returnvalue "Undefined" 0 0)
          (bind _returnvalue_2 (Effects|SpawnEmitteratLocation "/Game/StarterContent/Particles/P_Sparks.P_Sparks" (.Location (Math|Transform|BreakTransform _returnvalue))))
          (Utilities|FlowControl|Sequence
            (:then_0
              (Utilities|FlowControl|Delay 0.2)
              (Components|DestroyComponent _returnvalue_2))
            (:then_1
              (Audio|PlaySoundatLocation "/Game/Sonidos/laser2.laser2" (Transformation|GetActorLocation) "0, 0, 0" 1.0 1.0 0.0 0 0 0))))
        (:then_1
          (Utilities|FlowControl|Delay 0.5)
          (goto _label Reset))))))

(fn ConstructionScript)