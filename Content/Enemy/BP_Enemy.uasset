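; Melee enemy that chases the player, attacks at close range and is destroyed when its health runs out.
; On BeginPlay it finds the Jugador actor and starts a self-restarting AI MoveTo, which retries after a delay on failure.
; A looping timer checks range and plays the attack montage behind a DoOnce, calling Impactado on the player when it completes.
; Its own Impactado event reduces Vida by a fixed amount per hit.
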(event Custom|Impactado
  (CallFunction|ReducirVida 10)
  (if (<= (Variables|Default|GetVida) 0)
    (Actor|DestroyActor)))

(event Custom|FollowPlayer
  (bind _jugador (Variables|Default|GetJugador)
    (:then
      (AI|AIMoveTo self "0, 0, 0" _jugador 5e+01 false
        (:OnSuccess
          _)
        (:OnFail
          (Utilities|FlowControl|Delay 1.0)))
      (CallFunction|FollowPlayer))
    (:else)))

(event Custom|Attack
  (bind _jugador (Variables|Default|GetJugador)
    (:then
      (if (<= (Transformation|GetDistanceTo _jugador) 2e+02)
        (Utilities|FlowControl|DoOnce false :!label _label
          (:Completed
            (Animation|Montage|PlayMontage (Variables|Character|GetMesh) "/Game/Enemy/Enemy_Attack_AnimMontage.Enemy_Attack_AnimMontage"
              (:OnCompleted
                (Utilities|FlowControl|Sequence
                  (:then_0
                    (Default|Impactado (Variables|Default|GetJugador)))
                  (:then_1
                    (goto _label Reset)))))))))
    (:else)))

(event EventBeginPlay
  (bind _returnvalue (Actor|GetActorOfClass "/Game/Player/Jugador.Jugador_C"))
  (Variables|Default|SetJugador _returnvalue)
  (Utilities|FlowControl|Delay 0.1)
  (CallFunction|FollowPlayer)
  (Utilities|Time|SetTimerbyEvent (delegate Custom|Attack) 1.0 true))

(fn ConstructionScript
  (|CallParentFunction))